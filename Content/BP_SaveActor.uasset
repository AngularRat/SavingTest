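; BP_SaveActor is a test actor, apparently for saving, that creates, lists and clears generated test components.
; CreateComponent adds a component with fixed test values, and ClearGeneratedComponents removes them through inherited or external calls.
; ListComponents prints each component's ID and coordinates from both its DataStruct and DataObject in different colors, exposing both storage forms for comparison.
; The event graph and construction script are empty.
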(fn `ClearGeneratedComponents`
  (`self.ClearComponents`))

(fn `CreateComponent`
  (`self.CreateTestComponent` 1 2 3 4))

(fn `ListComponents`
  (locals (TestComponent :type "TestComponent Object Reference"))
  (bind _testcomponent (`local.TestComponent`))
  (bind _dataobject (`TestComponent.DataObject` _testcomponent))
  (bind (_datastruct_id _datastruct_x _datastruct_y _datastruct_z) (break `DataStruct` (`TestComponent.DataStruct` _testcomponent)))
  (for _array_element (`self.GeneratedComponents`)
    (set `local.TestComponent` _array_element)
    (`KismetSystemLibrary.PrintString` (`KismetTextLibrary.Conv_TextToString` (`|FormatText` "DS: id:{id} X:{x} Y:{y} Z:{z}" _datastruct_id _datastruct_x _datastruct_y _datastruct_z)) true true (struct :`R` 1.0 :`B` 0.9625 :`A` 1.0) 10.0)
    (`KismetSystemLibrary.PrintString` (`KismetTextLibrary.Conv_TextToString` (`|FormatText` "DO: id:{id} X:{x} Y:{y} Z:{z}" (`DataObject.Id` _dataobject) (`DataObject.X` _dataobject) (`DataObject.Y` _dataobject) (`DataObject.Z` _dataobject))) true true (struct :`R` 1.0 :`G` 0.376997 :`A` 1.0) 10.0)))

(fn `UserConstructionScript`)